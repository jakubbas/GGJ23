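; Test Blueprint, marked do-not-use, that stretches a spline with meshes along it to follow the player character.
; Every Tick it rebuilds the point list in world space, replacing only the last point with player 0's location.
; UpdateVisuals then destroys all spline mesh components and recreates one per segment from local-space locations and tangents, so components churn every frame.
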(event EventTick
  (params (DeltaSeconds :type Float%20%28single-precision%29))
  (bind _spline (Variables|Default|GetSpline))
  (bind _temppointarray (Variables|Default|GettempPointArray))
  (bind _returnvalue (Spline|GetNumberOfSplinePoints _spline))
  (bind _returnvalue_2 (- _returnvalue 1))
  ;[1 1 1] TEST DO NOT USE
  (for _index (range 0 _returnvalue_2)
    (if (== _index _returnvalue_2)
      (Utilities|Array|Add (Variables|Default|GettempPointArray) (Transformation|GetActorLocation (Game|GetPlayerCharacter 0)))
      (else
        (Utilities|Array|Add (Variables|Default|GettempPointArray) (Spline|GetLocationatSplinePoint (Variables|Default|GetSpline) _index "World")))))
  (if (> (Utilities|Array|Length _temppointarray) 0)
    (Spline|SetSplinePoints (Variables|Default|GetSpline) _temppointarray "World" true)
    (Utilities|Array|Clear (Variables|Default|GettempPointArray))
    (CallFunction|UpdateVisuals)))

(fn ConstructionScript)

(fn UpdateVisuals
  (bind _spline (Variables|Default|GetSpline))
  (for _array_element (Variables|Default|GetsplineMeshArray)
    (Components|DestroyComponent _array_element))
  (Utilities|Array|Clear (Variables|Default|GetsplineMeshArray))
  (for _index (range 0 (- (Spline|GetNumberOfSplinePoints (Variables|Default|GetSpline)) 2))
    (bind _returnvalue (AddComponent|AddSplineMeshComponent false))
    (SplineMesh|SetStartandEnd _returnvalue (.Location (Spline|GetLocationandTangentatSplinePoint _spline _index "Local")) (.Tangent (Spline|GetLocationandTangentatSplinePoint _spline _index "Local")) (.Location (Spline|GetLocationandTangentatSplinePoint _spline (+ _index 1) "Local")) (.Tangent (Spline|GetLocationandTangentatSplinePoint _spline (+ _index 1) "Local")) true :!class /Script/Engine.SplineMeshComponent)
    (Transformation|AttachComponentToComponent _returnvalue (Variables|Default|GetDefaultSceneRoot) "None" "KeepRelative" "KeepRelative" "KeepRelative" true)
    (Utilities|Array|Add (Variables|Default|GetsplineMeshArray) _returnvalue)))