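; BP_Tree is the tree actor that starts and resolves root growth runs in the game.
; Init caches the player and tree pawns, then spawns a BP_Root at a random point on a circle around the tree.
; The root is passed to the player via an interface message and initialised.
; When it finishes, finding water fires CallWaterFound and possesses the tree pawn; otherwise CallGameEnded fires.
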(event Custom|Init
  ;[1 1 1] TEST: Spawn first root
  (Variables|Default|Setplayer (Game|Player|GetPlayerPawn 0))
  (CallFunction|SpawnRoot)
  (bind _returnvalue (Actor|GetActorOfClass "/Game/Characters/Pawn_Tree.Pawn_Tree_C"))
  (Variables|Default|SettreePawn _returnvalue))

(event Custom|SpawnRoot
  ;[1 1 1] Creates and initialises root
  (bind (_rootstartposition _rootstartdirection) (CallFunction|GetRootSpawnPoint))
  (bind _returnvalue (Game|SpawnActorfromClass "/Game/Migrate/BP_Root.BP_Root_C" (Math|Transform|MakeTransform _rootstartposition) "AlwaysSpawn" 0 0))
  (bind _output_get (Variables|Default|SetcurrentRoot _returnvalue))
  (EventDispatchers|BindEventtoRootFinished _output_get (delegate Custom|EndRoot))
  (Class|BPIPlayer|ISetRoot(Message) (Variables|Default|Getplayer) _output_get)
  (Default|Init _output_get))

(event Custom|EndRoot
  (params (waterFound :type Boolean))
  ;[1 1 1] Root Ended
  (if waterFound
    (Default|CallWaterFound)
    (Pawn|Possess (Game|GetPlayerController 0) (Variables|Default|GettreePawn))
    (else
      (Default|CallGameEnded))))

(fn ConstructionScript)

(fn GetRootSpawnPoint
  (bind _returnvalue (Transformation|GetActorLocation))
  (bind (_x _y _z) (Class|KismetMathLibrary|BreakVector3f _returnvalue))
  (LocalVariables|Setrand (Math|Random|RandomFloatinRange 0.0 3.6e+02))
  (bind _output_get (LocalVariables|Setpos (Math|Vector|MakeVector (+ (* (Variables|Default|GetspawnRadius) (Math|Trig|Cos(Degrees) (LocalVariables|Getrand))) _x) (+ _y (* (Variables|Default|GetspawnRadius) (Math|Trig|Sin(Degrees) (LocalVariables|Getrand)))) _z)))
  (return (LocalVariables|Getpos) (Math|Rotator|FindLookatRotation (Transformation|GetActorLocation) _output_get)))