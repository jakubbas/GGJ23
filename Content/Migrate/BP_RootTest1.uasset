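; Test root actor that grows a spline-mesh trail meant to follow the player, with a debug-print lose message on touch.
; Init starts a timer adding segments, and EndRoot alternates with it to pause and resume growth.
; Tick moves the last spline point to PlayerPosition, whose graph is unwired, and stretches the newest mesh.
; Segments bind overlap once superseded, while the polling overlap check is disconnected.
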(event Custom|Init
  ;[1 1 1] Initialises the root
  (Utilities|Time|SetTimerbyEvent (delegate Custom|EndRoot) 5.0)
  (Variables|Default|SetplayerCharacter (Game|Player|GetPlayerPawn 0))
  (Utilities|Array|Add (Variables|Default|GetpointArray) (Transformation|GetActorLocation))
  (Utilities|Array|Add (Variables|Default|GetpointArray) (Transformation|GetActorLocation))
  (bind _returnvalue (Utilities|Time|SetTimerbyEvent (delegate Custom|MakeNewSegment) 1.0 true))
  (Variables|Default|SetsegmentCreationTimer _returnvalue)
  (Variables|Default|SetisActive true))

(event Custom|IsOverlapping
  ;[1 1 1] Lose Condition
)

(event Custom|EndRoot
  (Variables|Default|SetisActive false)
  (Utilities|Time|ClearandInvalidateTimerbyHandle (Variables|Default|GetsegmentCreationTimer))
  (Utilities|Time|SetTimerbyFunctionName 0 "Init" 5.0))

(event Custom|MakeNewSegment
  (bind _spline (Variables|Default|GetSpline))
  (bind _pointarray (Variables|Default|GetpointArray))
  (bind _pointarray_2 (Variables|Default|GetpointArray))
  (bind _returnvalue (Utilities|Array|Length _pointarray))
  (bind _returnvalue_2 (Utilities|Array|Length _pointarray_2))
  (bind _returnvalue_3 (- _returnvalue 1))
  (bind _returnvalue_4 (- _returnvalue 2))
  (bind (_location _tangent) (Spline|GetLocationandTangentatSplinePoint _spline _returnvalue_4 "World"))
  (bind (_location_2 _tangent_2) (Spline|GetLocationandTangentatSplinePoint _spline _returnvalue_3 "World"))
  ;[1 1 1] Makes a new segment in the spline and creates a new mesh
  (Development|PrintString "make new segment")
  (if (or (< _returnvalue_2 2) (!= (- _returnvalue_2 1) (- _returnvalue_2 2)))
    (Utilities|IsValid (Variables|Default|GetcurrentSplineMesh)
      (:Is%20Valid
        (Collision|BindEventtoOnComponentBeginOverlap (Variables|Default|GetcurrentSplineMesh) (delegate Custom|BeginOverlap)))
      (:Is%20Not%20Valid
        _))
    (Utilities|Array|Add (Variables|Default|GetpointArray) (Utilities|PlayerPosition))
    (bind _returnvalue_5 (AddComponent|AddSplineMeshComponent false))
    (Variables|Default|SetcurrentSplineMesh _returnvalue_5)
    (Utilities|Array|Add (Variables|Default|GetsplineMeshArray) _returnvalue_5)
    (SplineMesh|SetStartandEnd (Variables|Default|GetcurrentSplineMesh) _location _tangent _location_2 _tangent_2 true :!class /Script/Engine.SplineMeshComponent)
    (Transformation|AttachComponentToComponent (Variables|Default|GetcurrentSplineMesh) (Variables|Default|GetDefaultSceneRoot) "None" "SnapToTarget" "KeepRelative" "KeepRelative" true)))

(event Custom|BeginOverlap
  (params (OverlappedComponent :type Primitive%20Component%20Object%20Reference) (OtherActor :type Actor%20Object%20Reference) (OtherComp :type Primitive%20Component%20Object%20Reference) (OtherBodyIndex :type Integer) (bFromSweep :type Boolean) (SweepResult :type Hit%20Result%20Structure%20%28by%20ref%29))
  ;[1 1 1] Makes a new segment in the spline and creates a new mesh
  (if (== OtherActor (Variables|Default|GetplayerCharacter))
    (Development|PrintString "LOSER LOSER LOSER LOSER LOSER LOSER LOSER LOSER LOSER LOSER LOSER LOSER LOSER LOSER LOSER LOSER LOSER LOSER")))

(event EventTick
  (params (DeltaSeconds :type Float%20%28single-precision%29))
  (bind _pointarray (Variables|Default|GetpointArray))
  (bind _pointarray_2 (Variables|Default|GetpointArray))
  (bind _spline (Variables|Default|GetSpline))
  (bind _returnvalue (Utilities|Array|Length _pointarray_2))
  (bind _returnvalue_2 (- _returnvalue 1))
  (bind _returnvalue_3 (- _returnvalue 2))
  (bind (_location _tangent) (Spline|GetLocationandTangentatSplinePoint _spline _returnvalue_3 "World"))
  (bind (_location_2 _tangent_2) (Spline|GetLocationandTangentatSplinePoint _spline _returnvalue_2 "World"))
  ;[1 1 1] Updates the end of the spline to the player position
  (CallFunction|IsOverlapping)
  (if (Variables|Default|GetisActive)
    (Utilities|Array|SetArrayElem _pointarray (- (Utilities|Array|Length _pointarray) 1) (Utilities|PlayerPosition))
    (Spline|SetSplinePoints (Variables|Default|GetSpline) (Variables|Default|GetpointArray) "World" true)
    (Utilities|IsValid (Variables|Default|GetcurrentSplineMesh)
      (:Is%20Valid
        (SplineMesh|SetStartandEnd (Variables|Default|GetcurrentSplineMesh) _location _tangent _location_2 _tangent_2 true :!class /Script/Engine.SplineMeshComponent)))))

(fn ConstructionScript)