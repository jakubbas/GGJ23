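; Actor component that hides world objects blocking the camera's view of its owning player.
; Init stores the owner and camera, and CameraBlockerUpdate unhides the previous blockers before running a multi object trace from camera to owner.
; Static and dynamic hits are hidden and tracked in TransparentList unless their DontHideMessage call opts out.
; Actors are hidden outright rather than faded, and the trace draws debug lines each call.
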(event Custom|Init
  (params (owner :type Actor%20Object%20Reference) (camera :type Camera%20Component%20Object%20Reference))
  (Variables|Default|Setowner owner)
  (Variables|Default|Setcamera camera))

(fn CameraBlockerUpdate
  ;[1 1 1] Culls the assets currently blocking the player
  (for _array_element (Variables|Default|GettransparentList)
    (Rendering|SetActorHiddenInGame _array_element false))
  (Utilities|Array|Clear (Variables|Default|GettransparentList))
  (bind (_outhits _returnvalue) (Class|KismetSystemLibrary|LineTraceMultiforObjects (Transformation|GetWorldLocation (Variables|Default|Getcamera)) (Transformation|GetActorLocation (Variables|Default|Getowner)) (Utilities|Array|MakeArray "ObjectTypeQuery1" "ObjectTypeQuery2") false 0 "ForOneFrame" true))
  (if _returnvalue
    (for _array_element_2 _outhits
      (bind _donthide (Class|BPIAssetDontHide|DontHide(Message) (.HitActor (Collision|BreakHitResult _array_element_2))))
      (if (not _donthide)
        (Utilities|Array|AddUnique (Variables|Default|GettransparentList) (.HitActor (Collision|BreakHitResult _array_element_2)))
        (Rendering|SetActorHiddenInGame (.HitActor (Collision|BreakHitResult _array_element_2)) true)))))