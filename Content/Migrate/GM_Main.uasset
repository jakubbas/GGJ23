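; Main game mode that starts the tree-based game and tracks how much water has been found.
; On BeginPlay it initializes the BP_Tree actor, binds to its water-found and game-ended events, and creates the viewport HUD.
; Each water find increments a counter, sent to the HUD as a clamped fraction of the maximum.
; Game end only prints a message, and PostGame is an empty stub.
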(event Custom|GameEnd
  (Development|PrintString "GAME FINISHED"))

(event Custom|BeginGame
  ;[1 1 1] Initialises tree
  (Class|BPIPC|IInit(Message) (Game|GetPlayerController 0)) ; Doesnt use custom player controller yet, does nothing
  (bind _returnvalue (Actor|GetActorOfClass "/Game/Migrate/BP_Tree.BP_Tree_C"))
  (Default|Init _returnvalue)
  (EventDispatchers|BindEventtoWaterFound _returnvalue (delegate Custom|WaterFound))
  (EventDispatchers|AssignGameEnded _returnvalue (EventDispatchers|CreateEvent :!event Custom|GameEnd))
  (bind _returnvalue_2 (UserInterface|CreateWidget "/Game/UserInterface/UI_Viewport.UI_Viewport_C" (Game|GetPlayerController 0)))
  (UserInterface|Viewport|AddtoViewport _returnvalue_2 0)
  (Variables|Default|SetHUD _returnvalue_2))

(event Custom|WaterFound
  ;[1 1 1] Adds water, clamps it to 0-1 and passes to HUD.
  (bind _result (Math|Integer|IncrementInt (Variables|Default|Getwater))
    (:%20%20
      (Class|BPIHUD|ISetPercent(Message) (Variables|Default|GetHUD) (Math|Float|MapRangeClamped (Math|Conversions|ToFloat(Integer) _result) 0.0 (Math|Conversions|ToFloat(Integer) (Variables|Default|GetmaxWater)) 0.0 1.0)))))

(event Custom|PostGame)

(event EventBeginPlay
  (CallFunction|BeginGame))

(fn ConstructionScript)